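; BP_Ninja is an auto-running player character that moves forward every tick while the MoveRight axis steers it sideways.
; SwapControlEvent inverts that steering for a given time, using a retriggerable delay so repeat calls restart the countdown.
; BeginPlay records the starting X and adds the main HUD widget to the viewport.
; Tick updates Distance from X travel since the start, divided by 100.
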(event Custom|SwapControlEvent
  (params (Time :type Float%20%28double-precision%29))
  (Variables|Default|SetSwapControl true)
  (Utilities|FlowControl|RetriggerableDelay Time)
  (Variables|Default|SetSwapControl false))

(event EventBeginPlay
  (bind _output_get (Variables|Default|SetInitialLocation (.x (Transformation|GetActorLocation))))
  (bind _returnvalue (UserInterface|CreateWidget "/Game/Scripting/UI/UI_MainHUD.UI_MainHUD_C"))
  (UserInterface|Viewport|AddtoViewport _returnvalue 0)
  (Variables|Default|SetMainHUD _returnvalue))

(event EventTick
  (params (DeltaSeconds :type Float%20%28single-precision%29))
  (Pawn|Input|AddMovementInput (Transformation|GetActorForwardVector) 1.0 false)
  (Variables|Default|SetDistance (/ (- (.x (Transformation|GetActorLocation)) (stale EventBeginPlay _output_get)) 1e+02)))

(event Input|AxisEvents|InputAxisMoveRight
  (params (AxisValue :type Float%20%28single-precision%29))
  (bind _returnvalue (Pawn|GetControlRotation :!class /Script/Engine.Pawn))
  (if (Variables|Default|GetSwapControl)
    (Variables|Default|SetSwapAxisValue -1.0)
    (else
      (Variables|Default|SetSwapAxisValue 1.0)))
  (Pawn|Input|AddMovementInput (Math|Vector|GetRightVector (Math|Rotator|MakeRotator (.roll _returnvalue) 0.0 (.yaw _returnvalue))) (* AxisValue (Variables|Default|GetSwapAxisValue)) false))

(fn ConstructionScript)