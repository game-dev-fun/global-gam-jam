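; BP_SpawnPoint is a spawner that places an actor of SpawnClass on the surface of a surrounding BP_Roots actor.
; On BeginPlay it fires one visibility line trace of LineTraceLength in a random direction perpendicular to its forward vector.
; If the trace hits BP_Roots, it spawns the actor at the impact, with rotation built from the hit normal and pitched back 90 degrees.
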(event EventBeginPlay
  (bind _returnvalue (Transformation|GetActorLocation))
  (bind (_outhit _returnvalue_2) (Collision|LineTraceByChannel _returnvalue (+ _returnvalue (* (Math|Vector|Normalize (Math|Vector|ProjectVectorontoPlane (Math|Random|RandomUnitVector) (Transformation|GetActorForwardVector))) (Variables|Default|GetLineTraceLength))) "TraceTypeQuery1" false 0 "None" true "(R=1.000000,G=0.000000,B=0.000000,A=1.000000)" "(R=0.000000,G=1.000000,B=0.000000,A=1.000000)" 2e+01))
  (if _returnvalue_2
    (Utilities|Casting|CastToBP_Roots (.HitActor (Collision|BreakHitResult _outhit)))
    (Game|SpawnActorfromClass (Variables|Default|GetSpawnClass) (Math|Transform|MakeTransform (.Location (Collision|BreakHitResult _outhit)) (Math|Rotator|MakeRotator (.roll (Math|Rotator|MakeRotationfromAxes (.Normal (Collision|BreakHitResult _outhit)) "0, 0, 0" "0, 0, 0")) (- (.pitch (Math|Rotator|MakeRotationfromAxes (.Normal (Collision|BreakHitResult _outhit)) "0, 0, 0" "0, 0, 0")) 9e+01) (.yaw (Math|Rotator|MakeRotationfromAxes (.Normal (Collision|BreakHitResult _outhit)) "0, 0, 0" "0, 0, 0"))) "1.000000,1.000000,1.000000") "Undefined" 0 0)))

(fn ConstructionScript)