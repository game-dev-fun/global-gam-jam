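; BP_Roots is a track segment that extends the level as BP_Ninja advances, then removes itself.
; Construction fits the mesh offset and end trigger to the mesh's length, and BeginPlay spawns a BP_SpawnPoint for BP_SwapControls at a padded random X along it.
; Ninja overlap tells BP_GameMode to add a root, then after a delay runs cleanup of swap controls and spawn points, filtered by XLessThanActor, whose X comparison is unconnected.
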(event OnComponentBeginOverlap(Box)
  (params (OverlappedComponent :type Primitive%20Component%20Object%20Reference) (OtherActor :type Actor%20Object%20Reference) (OtherComp :type Primitive%20Component%20Object%20Reference) (OtherBodyIndex :type Integer) (bFromSweep :type Boolean) (SweepResult :type Hit%20Result%20Structure%20%28by%20ref%29))
  (Utilities|Casting|CastToBP_Ninja OtherActor)
  (bind _asbp_game_mode (Utilities|Casting|CastToBP_GameMode (Game|GetGameMode)))
  (Default|AddRoot _asbp_game_mode 1)
  (CallFunction|DestroySpawnedActors))

(event Custom|DestroySpawnedActors
  (Utilities|FlowControl|Delay 2.0)
  (CallFunction|DestroySwapControls)
  (CallFunction|DestroySpawnPoints)
  (Actor|DestroyActor))

(event EventBeginPlay
  (bind _returnvalue (Transformation|GetActorLocation))
  (Game|SpawnActorfromClass "/Game/Scripting/BP_Classes/BP_SpawnPoint.BP_SpawnPoint_C" (Math|Transform|MakeTransform (Math|Vector|MakeVector (Math|Random|RandomFloatinRange (+ (.x _returnvalue) (Variables|Default|GetPadding)) (- (+ (.x _returnvalue) (Variables|Default|GetLength)) (Variables|Default|GetPadding))) (.y _returnvalue) (.z _returnvalue)) "0, 0, 0" "1.000000,1.000000,1.000000") "Undefined" 0 "/Game/Scripting/BP_Classes/BP_SwapControls.BP_SwapControls_C" 3e+02 0))

(fn ConstructionScript
  (bind _staticmesh (Variables|Default|GetStaticMesh))
  (bind (_min _max) (Components|StaticMesh|GetLocalBounds _staticmesh))
  (bind _output_get (Variables|Default|SetLength (- (.x _max) (.x _min))))
  (Transformation|SetRelativeLocation (Variables|Default|GetStaticMesh) (Math|Vector|MakeVector (/ _output_get 2.0) 0.0 0.0) false false)
  (Transformation|SetRelativeTransform (Variables|Default|GetBox) (Math|Transform|MakeTransform (Math|Vector|MakeVector _output_get 0.0 0.0) "0, 0, 0" "1.000000,6.000000,6.000000") false false))

(fn DestroySwapControls
  (bind _outactors (Actor|GetAllActorsOfClass "/Game/Scripting/BP_Classes/BP_SwapControls.BP_SwapControls_C"))
  (for _array_element _outactors
    (if (Utilities|XLessThanActor (.x (Transformation|GetActorLocation _array_element)))
      (Actor|DestroyActor _array_element))))

(fn DestroySpawnPoints
  (bind _outactors (Actor|GetAllActorsOfClass "/Game/Scripting/BP_Classes/BP_SpawnPoint.BP_SpawnPoint_C"))
  (for _array_element _outactors
    (if (Utilities|XLessThanActor (.x (Transformation|GetActorLocation _array_element)))
      (Actor|DestroyActor _array_element))))