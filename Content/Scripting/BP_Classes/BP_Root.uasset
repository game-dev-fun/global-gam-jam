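; BP_Root is an actor that lays out a static mesh and a box component along its local X axis.
; The construction script measures the mesh's local-bounds length, shifts the mesh forward by half of it, and places the box at the full length with enlarged Y and Z scale.
; A random material color call is left unconnected, and the actor has no runtime logic.
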(event EventBeginPlay)

(fn ConstructionScript
  (bind _staticmesh (Variables|Default|GetStaticMesh))
  (bind (_min _max) (Components|StaticMesh|GetLocalBounds _staticmesh))
  (bind _output_get (Variables|Default|SetLength (- (.x _max) (.x _min))))
  (Transformation|SetRelativeLocation (Variables|Default|GetStaticMesh) (Math|Vector|MakeVector (/ _output_get 2.0) 0.0 0.0) false false)
  (Transformation|SetRelativeTransform (Variables|Default|GetBox) (Math|Transform|MakeTransform (Math|Vector|MakeVector _output_get 0.0 0.0) "0, 0, 0" "1.000000,6.000000,6.000000") false false))