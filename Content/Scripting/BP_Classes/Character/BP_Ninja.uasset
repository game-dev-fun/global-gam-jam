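; Player ninja character for an endless-runner style game that runs forward automatically and steers sideways through the MoveRight axis.
; Timed debuff events block left or right turns or invert steering, attaching emitters to legs or head until a RetriggerableDelay expires.
; Tick measures distance along world X, saves any new record to the HighScoreSlot save and plays the HUD high-score animation once.
; BeginPlay creates the HUD and loads the stored record.
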(event Custom|SwapControlEvent
  (params (Time :type Float%20%28double-precision%29))
  (if (Variables|Default|GetSwapControl)
    _
    (else
      (bind _returnvalue (Game|SpawnActorfromClass "/Game/Scripting/BP_Classes/SpawnActors/Emitter/BP_Emitter_Head.BP_Emitter_Head_C" (Math|Transform|MakeTransform "0, 0, 0" "0, 0, 0" "1.000000,1.000000,1.000000") "Undefined" 0 0))
      (Transformation|AttachComponentToComponent _returnvalue (Variables|Character|GetMesh) "head" "KeepRelative" "KeepRelative" "KeepRelative" true)))
  (Variables|Default|SetSwapControl true)
  (Utilities|FlowControl|RetriggerableDelay Time)
  (Variables|Default|SetSwapControl false)
  (Actor|DestroyActor _returnvalue))

(event Custom|TurnLeftOffEvent
  (params (Time :type Float%20%28double-precision%29))
  (if (Variables|Default|GetTurnLeftOff)
    _
    (else
      (bind _returnvalue (Game|SpawnActorfromClass "/Game/Scripting/BP_Classes/SpawnActors/Emitter/BP_Emitter_Calf_L.BP_Emitter_Calf_L_C" (Math|Transform|MakeTransform "0, 0, 0" "0, 0, 0" "1.000000,1.000000,1.000000") "Undefined" 0 0))
      (Transformation|AttachComponentToComponent _returnvalue (Variables|Character|GetMesh) "calf_l" "SnapToTarget" "SnapToTarget" "SnapToTarget" true)
      (bind _returnvalue_2 (Game|SpawnActorfromClass "/Game/Scripting/BP_Classes/SpawnActors/Emitter/BP_Emitter_Thigh_L.BP_Emitter_Thigh_L_C" (Math|Transform|MakeTransform "0, 0, 0" "0, 0, 0" "1.000000,1.000000,1.000000") "Undefined" 0 0))
      (Transformation|AttachComponentToComponent _returnvalue_2 (Variables|Character|GetMesh) "thigh_l" "SnapToTarget" "SnapToTarget" "SnapToTarget" true)))
  (Variables|Default|SetTurnLeftOff true)
  (Utilities|FlowControl|RetriggerableDelay Time)
  (Variables|Default|SetTurnLeftOff false)
  (Actor|DestroyActor _returnvalue)
  (Actor|DestroyActor _returnvalue_2))

(event Custom|TurnRightOffEvent
  (params (Time :type Float%20%28double-precision%29))
  (if (Variables|Default|GetTurnRightOff)
    _
    (else
      (bind _returnvalue (Game|SpawnActorfromClass "/Game/Scripting/BP_Classes/SpawnActors/Emitter/BP_Emitter_Thigh_R.BP_Emitter_Thigh_R_C" (Math|Transform|MakeTransform "0, 0, 0" "0, 0, 0" "1.000000,1.000000,1.000000") "Undefined" 0 0))
      (Transformation|AttachComponentToComponent _returnvalue (Variables|Character|GetMesh) "thigh_r" "SnapToTarget" "SnapToTarget" "SnapToTarget" true)
      (bind _returnvalue_2 (Game|SpawnActorfromClass "/Game/Scripting/BP_Classes/SpawnActors/Emitter/BP_Emitter_Calf_R.BP_Emitter_Calf_R_C" (Math|Transform|MakeTransform "0, 0, 0" "0, 0, 0" "1.000000,1.000000,1.000000") "Undefined" 0 0))
      (Transformation|AttachComponentToComponent _returnvalue_2 (Variables|Character|GetMesh) "calf_r" "SnapToTarget" "SnapToTarget" "SnapToTarget" true)))
  (Variables|Default|SetTurnRightOff true)
  (Utilities|FlowControl|RetriggerableDelay Time)
  (Variables|Default|SetTurnRightOff false)
  (Actor|DestroyActor _returnvalue)
  (Actor|DestroyActor _returnvalue_2))

(event EventBeginPlay
  (bind _returnvalue (Game|GetPlayerController 0))
  (Variables|/Script/Engine.PlayerController|SetbShowMouseCursor _returnvalue false)
  (Input|SetInputModeGameOnly _returnvalue false)
  (bind _output_get (Variables|Default|SetInitialLocation (.x (Transformation|GetActorLocation))))
  (bind _returnvalue_2 (UserInterface|CreateWidget "/Game/Scripting/UI/UI_MainHUD.UI_MainHUD_C"))
  (UserInterface|Viewport|AddtoViewport _returnvalue_2 0)
  (Variables|Default|SetMainHUD _returnvalue_2)
  (bind _returnvalue_3 (SaveGame|DoesSaveGameExist "HighScoreSlot"))
  (if _returnvalue_3
    (bind _returnvalue_4 (SaveGame|LoadGamefromSlot "HighScoreSlot"))
    (bind _assg_high_score (Utilities|Casting|CastToSG_HighScore _returnvalue_4))
    (Variables|Default|SetMaxDistance (Variables|/Game/Scripting/Save/SG_HighScore.SG_HighScore_C|GetHighScore _assg_high_score))))

(event EventTick
  (params (DeltaSeconds :type Float%20%28single-precision%29))
  (Pawn|Input|AddMovementInput (Transformation|GetActorForwardVector) 1.0 false)
  (bind _output_get (Variables|Default|SetDistance (/ (- (.x (Transformation|GetActorLocation)) (stale EventBeginPlay _output_get)) 1e+02)))
  (if (> _output_get (Variables|Default|GetMaxDistance))
    (Variables|Default|SetMaxDistance _output_get)
    (CallFunction|SaveHighScore)
    (Utilities|FlowControl|DoOnce false
      (:Completed
        (Default|PlayHighScoreAnimation (Variables|Default|GetMainHUD))))))

(event Input|AxisEvents|InputAxisMoveRight
  (params (AxisValue :type Float%20%28single-precision%29))
  (bind _returnvalue (Pawn|GetControlRotation :!class /Script/Engine.Pawn))
  (if (Variables|Default|GetSwapControl)
    (Variables|Default|SetSwapAxisValue -1.0)
    (else
      (Variables|Default|SetSwapAxisValue 1.0)))
  (if (not (and (> (* AxisValue (Variables|Default|GetSwapAxisValue)) 0.0) (Variables|Default|GetTurnRightOff)))
    (if (not (and (< (* AxisValue (Variables|Default|GetSwapAxisValue)) 0.0) (Variables|Default|GetTurnLeftOff)))
      (Pawn|Input|AddMovementInput (Math|Vector|GetRightVector (Math|Rotator|MakeRotator (.roll _returnvalue) 0.0 (.yaw _returnvalue))) (* AxisValue (Variables|Default|GetSwapAxisValue)) false))))

(fn ConstructionScript)

(fn SaveHighScore
  (bind _maxdistance (Variables|Default|GetMaxDistance))
  (bind _returnvalue (SaveGame|DoesSaveGameExist "HighScoreSlot"))
  (if _returnvalue
    (bind _returnvalue_2 (SaveGame|LoadGamefromSlot "HighScoreSlot"))
    (bind _assg_high_score (Utilities|Casting|CastToSG_HighScore _returnvalue_2))
    (Variables|/Game/Scripting/Save/SG_HighScore.SG_HighScore_C|SetHighScore _assg_high_score _maxdistance)
    (SaveGame|SaveGametoSlot _assg_high_score "HighScoreSlot")
    (else
      (bind _returnvalue_3 (SaveGame|CreateSaveGameObject "/Game/Scripting/Save/SG_HighScore.SG_HighScore_C"))
      (Variables|/Game/Scripting/Save/SG_HighScore.SG_HighScore_C|SetHighScore _returnvalue_3 _maxdistance)
      (SaveGame|SaveGametoSlot _returnvalue_3 "HighScoreSlot"))))